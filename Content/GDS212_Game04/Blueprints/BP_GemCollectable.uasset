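; BP_GemCollectable is a gem pickup that adds one point to the player's score.
; On BeginPlay it caches player 0's BP_FirstPersonCharacter.
; When its sphere collision is overlapped, it prints a +1 debug message, increments that character's CurrentScore, plays the gem sound and destroys itself.
; The overlap handler does not check which actor overlapped, so any overlap credits the cached player.
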(event OnComponentBeginOverlap(SphereCollision)
  (params (OverlappedComponent :type Primitive%20Component%20Object%20Reference) (OtherActor :type Actor%20Object%20Reference) (OtherComp :type Primitive%20Component%20Object%20Reference) (OtherBodyIndex :type Integer) (bFromSweep :type Boolean) (SweepResult :type Hit%20Result%20Structure%20%28by%20ref%29))
  (Development|PrintString "+1" true true "(R=1.000000,G=0.782595,B=0.000000,A=1.000000)")
  (Variables|/Game/FirstPerson/Blueprints/BP_FirstPersonCharacter.BP_FirstPersonCharacter_C|SetCurrentScore (Variables|Default|GetAs%20BP%20First%20Person%20Character) (+ (Variables|/Game/FirstPerson/Blueprints/BP_FirstPersonCharacter.BP_FirstPersonCharacter_C|GetCurrentScore (Variables|Default|GetAs%20BP%20First%20Person%20Character)) 1))
  (Audio|PlaySound2D "/Game/GDS212_Game04/SFX/SC_GemGet_Cue.SC_GemGet_Cue" 1.0 1.0 0.0 0 0)
  (Actor|DestroyActor))

(event EventBeginPlay
  (bind _asbp_first_person_character (Utilities|Casting|CastToBP_FirstPersonCharacter (Game|GetPlayerCharacter 0)))
  (Variables|Default|SetAs%20BP%20First%20Person%20Character _asbp_first_person_character))

(event EventTick
  (params (DeltaSeconds :type Float%20%28single-precision%29)))

(fn ConstructionScript)